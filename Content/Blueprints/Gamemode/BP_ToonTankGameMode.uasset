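; Game mode Blueprint for ToonTank that handles the match UI for game start, player HP and game end.
; StartGame adds the start-game and HP display widgets to the viewport, and GetHP writes the received HP value into the display's text.
; GameOver clears all widgets, then shows a game-over widget with a win or lose message based on its WinGame input.
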(event EventGameOver
  (params (bWinGame :type Boolean))
  (Viewport|RemoveAllWidgets)
  (bind _returnvalue (UserInterface|CreateWidget "/Game/Blueprints/Widget/WBP_GameOverWidget.WBP_GameOverWidget_C"))
  (UserInterface|Viewport|AddtoViewport _returnvalue 0)
  (Rendering|Components|TextRender|SetText (Variables|/Game/Blueprints/Widget/WBP_GameOverWidget.WBP_GameOverWidget_C|GetDisplaytext _returnvalue) (select bWinGame "You win !" "You lose !")))

(event EventGetHP
  (params (fHP :type Float%20%28single-precision%29))
  (Rendering|Components|TextRender|SetText (Variables|/Game/Blueprints/Widget/WBP_HPDisplay.WBP_HPDisplay_C|GetDisplayHP (stale EventStartGame _returnvalue_2)) (Utilities|Text|ToText(Float) fHP "HalfToEven")))

(event EventStartGame
  (bind _returnvalue (UserInterface|CreateWidget "/Game/Blueprints/Widget/WBP_StartGameWidget.WBP_StartGameWidget_C"))
  (UserInterface|Viewport|AddtoViewport _returnvalue 0)
  (bind _returnvalue_2 (UserInterface|CreateWidget "/Game/Blueprints/Widget/WBP_HPDisplay.WBP_HPDisplay_C"))
  (UserInterface|Viewport|AddtoViewport _returnvalue_2 0))

(fn ConstructionScript)